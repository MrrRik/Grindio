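; Manager that periodically triggers enemy waves from every EnemySpawner actor in the level, up to a maximum count.
; Tick passes through a DoOnce that is reset after a NextWaveTimer delay, forming a repeating wave loop.
; Each pass calls SpawnEnemyWave on spawners while TotalEnemies stays within MaxEnemies, adding one per call.
; This graph never decrements that count.
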(event EventTick
  (params (DeltaSeconds :type Float%20%28single-precision%29))
  (Utilities|FlowControl|DoOnce false :!label _label
    (:Completed
      (bind _outactors (Actor|GetAllActorsOfClass "/Game/Gameplay/Blueprints/Enemies/EnemySpawner.EnemySpawner_C"))
      (for _array_element _outactors
        (if (<= (+ (Variables|Default|GetTotalEnemies) 1) (Variables|Default|GetMaxEnemies))
          (Default|SpawnEnemyWave _array_element)
          (Variables|Default|SetTotalEnemies (+ (Variables|Default|GetTotalEnemies) 1))))
      (Utilities|FlowControl|Delay (Variables|Default|GetNextWaveTimer))
      (goto _label Reset))))

(fn ConstructionScript)