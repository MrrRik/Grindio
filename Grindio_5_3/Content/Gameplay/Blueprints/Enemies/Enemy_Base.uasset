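; Base enemy character that roams the navmesh, chases the hero inside its far collider and stops to attack inside the near one, recoloring a range indicator per state.
; Contact damages the hero on a timer-reset cooldown; incoming damage spawns damage numbers and updates the health widget.
; Tick handles lock-on visibility and death, which drops a coin or rare health pickup and updates EnemySpawnManager counters.
; Construction applies configurable mesh and anim class.
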(event OnComponentHit(Mesh)
  (params (HitComponent :type Primitive%20Component%20Object%20Reference) (OtherActor :type Actor%20Object%20Reference) (OtherComp :type Primitive%20Component%20Object%20Reference) (NormalImpulse :type Vector :default "0, 0, 0") (Hit :type Hit%20Result%20Structure%20%28by%20ref%29))
  ;[0 0 0] Enemy Collides with hero Damage
  (if (== (Utilities|GetClass OtherActor) "/Game/Gameplay/Blueprints/Hero/Hero.Hero_C")
    (Utilities|FlowControl|DoOnce false
      (:Completed
        (bind _ashero (Utilities|Casting|CastToHero OtherActor))
        (Default|HeroDealtDamage _ashero true (Variables|Default|GetDamage))
        (Utilities|Time|SetTimerbyEvent (delegate Custom|DamageRate) (Variables|Default|GetAttackRate))))))

(event OnComponentBeginOverlap(nearbyCol)
  (params (OverlappedComponent :type Primitive%20Component%20Object%20Reference) (OtherActor :type Actor%20Object%20Reference) (OtherComp :type Primitive%20Component%20Object%20Reference) (OtherBodyIndex :type Integer) (bFromSweep :type Boolean) (SweepResult :type Hit%20Result%20Structure%20%28by%20ref%29))
  ;[1 1 1] If close hero detection
  (Variables|Default|SetAttacking true)
  (Rendering|Material|SetVectorParameterValue (Variables|Default|GetDMI_Range) "Color" "(R=1.000000,G=0.000000,B=0.000000,A=1.000000)" :!class /Script/Engine.MaterialInstanceDynamic))

(event OnComponentEndOverlap(nearbyCol)
  (params (OverlappedComponent :type Primitive%20Component%20Object%20Reference) (OtherActor :type Actor%20Object%20Reference) (OtherComp :type Primitive%20Component%20Object%20Reference) (OtherBodyIndex :type Integer))
  ;[1 1 1] If close hero detection
  (Utilities|FlowControl|Delay 2.6)
  (Variables|Default|SetAttacking false)
  (CallFunction|ChasePlayer OtherActor))

(event OnComponentBeginOverlap(FarCol)
  (params (OverlappedComponent :type Primitive%20Component%20Object%20Reference) (OtherActor :type Actor%20Object%20Reference) (OtherComp :type Primitive%20Component%20Object%20Reference) (OtherBodyIndex :type Integer) (bFromSweep :type Boolean) (SweepResult :type Hit%20Result%20Structure%20%28by%20ref%29))
  ;[1 1 1] Far away hero detection
  (CallFunction|ChasePlayer OtherActor))

(event OnComponentEndOverlap(FarCol)
  (params (OverlappedComponent :type Primitive%20Component%20Object%20Reference) (OtherActor :type Actor%20Object%20Reference) (OtherComp :type Primitive%20Component%20Object%20Reference) (OtherBodyIndex :type Integer))
  ;[1 1 1] Far away hero detection
  (CallFunction|Roam))

(event Custom|Roam
  ;[1 1 1] Roaming event
  (Rendering|Material|SetVectorParameterValue (Variables|Default|GetDMI_Range) "Color" "(R=0.000000,G=0.897796,B=1.000000,A=1.000000)" :!class /Script/Engine.MaterialInstanceDynamic)
  (bind _randomlocation (Class|NavigationSystemV1|GetRandomLocationinNavigableRadius (Transformation|GetActorLocation) (Variables|Default|Getradius) 0 0))
  (AI|AIMoveTo self _randomlocation 0 5.0 false
    (:OnSuccess
      (Utilities|FlowControl|Delay 1.0)
      (CallFunction|Roam))))

(event Custom|LootDecider
  ;[1 1 1] Decides which loot and where to spawn
  (bind _randomlocation (Class|NavigationSystemV1|GetRandomLocationinNavigableRadius (Transformation|GetWorldLocation (Variables|Default|GetStaticMesh1)) (Variables|Default|GetLootSpawnRadius) 0 0))
  (Development|PrintString (Utilities|String|ToString(Vector) _randomlocation))
  (bind _output_get (Variables|Default|SetLootLocation _randomlocation))
  (bind _output_get_2 (Variables|Default|SetGetHealthPickup (> (Math|Random|RandomIntegerinRange 0 10) 9)))
  (if _output_get_2
    (Game|SpawnActorfromClass "/Game/Gameplay/Blueprints/Gameplay/Pickup_Health.Pickup_Health_C" (Math|Transform|MakeTransform _output_get "0, 0, 0" "1.000000,1.000000,1.000000") "AlwaysSpawn" "OverrideRootScale" 0 0)
    (else
      (Game|SpawnActorfromClass "/Game/Gameplay/Blueprints/Gameplay/Pickup_Coin.Pickup_Coin_C" (Math|Transform|MakeTransform _output_get "0, 0, 0" "1.000000,1.000000,1.000000") "AlwaysSpawn" "OverrideRootScale" 0 0))))

(event Custom|DamageRate
  ;[0 0 0] Enemy Collides with hero Damage
  (Utilities|FlowControl|DoOnce false) ; enters at Reset
)

(event Custom|ChasePlayer
  (params (Player :type Actor%20Object%20Reference))
  ;[1 1 1] Chasing player event
  (Rendering|Material|SetVectorParameterValue (Variables|Default|GetDMI_Range) "Color" "(R=1.000000,G=0.341622,B=0.000000,A=1.000000)" :!class /Script/Engine.MaterialInstanceDynamic)
  (AI|AIMoveTo self "0, 0, 0" Player 1.5e+02 false
    (:OnSuccess
      (Utilities|FlowControl|Delay 1.0)
      (CallFunction|ChasePlayer))))

(event Custom|EnemyDealtDamage
  (params (Condition :type Boolean) (Damage :type Float%20%28double-precision%29))
  ;[0 0 0] Enemy has been dealt damage
  (if (and Condition (Variables|Default|GetHittable))
    (Variables|Default|SetHittable false)
    ;;[0.1667 0.1667 0.1667] Spawn damage numbers
    (bind _returnvalue (Game|ConstructObjectfromClass "/Game/Gameplay/UI/DamageNumbers.DamageNumbers_C" self Damage))
    (UserInterface|Viewport|AddtoViewport _returnvalue 0)
    (Variables|Default|SetCurrentHealth (- (Variables|Default|GetCurrentHealth) Damage))
    (bind _asenemy_hud (Utilities|Casting|CastToEnemy_HUD (UserInterface|GetUserWidgetObject (Variables|Default|GetEnemyHealthUI))))
    (Variables|/Game/Gameplay/UI/Enemy_HUD.Enemy_HUD_C|SetCurrentHealth_UI _asenemy_hud (Variables|Default|GetCurrentHealth))
    (Variables|Default|SetHittable true)
    (Variables|Default|SetGotHit false)))

(event EventBeginPlay
  ;[1 1 1] Set max hp and start roaming
  (Utilities|FlowControl|Sequence
    (:then_0
      (CallFunction|Roam))
    (:then_1
      (Variables|Default|SetCurrentHealth (Variables|Default|GetMaxHealth))
      (Variables|/Game/Gameplay/UI/Enemy_HUD.Enemy_HUD_C|SetMaxHealth_UI (.AsEnemy%20HUD (Utilities|Casting|CastToEnemy_HUD (UserInterface|GetUserWidgetObject (Variables|Default|GetEnemyHealthUI)))) (Variables|Default|GetMaxHealth)))))

(event EventTick
  (params (DeltaSeconds :type Float%20%28single-precision%29))
  (bind _currenthealth (Variables|Default|GetCurrentHealth))
  (bind _returnvalue (<= _currenthealth 0.0))
  (Utilities|FlowControl|Sequence
    (:then_0
      ;[1 1 1] Dying
      (if _returnvalue
        (Utilities|FlowControl|DoOnce false
          (:Completed
            (Variables|Default|SetLockedOn false)
            (Components|Activation|Activate (Variables|Default|GetPS_CoinSpray) false)
            (Utilities|FlowControl|Delay 0.3)
            (CallFunction|LootDecider)
            (Effects|SpawnEmitteratLocation "/Game/Gameplay/Effects/PS_Smoke.PS_Smoke" (- (Transformation|GetWorldLocation (Variables|Default|GetStaticMesh1)) "0, 0,-6.500000"))
            (Utilities|FlowControl|Delay 0.7)
            (bind _returnvalue_2 (Actor|GetActorOfClass "/Game/Gameplay/Blueprints/Enemies/EnemySpawnManager.EnemySpawnManager_C"))
            (Variables|/Game/Gameplay/Blueprints/Enemies/EnemySpawnManager.EnemySpawnManager_C|SetTotalEnemies _returnvalue_2 (- (Variables|/Game/Gameplay/Blueprints/Enemies/EnemySpawnManager.EnemySpawnManager_C|GetTotalEnemies _returnvalue_2) 1))
            (Variables|/Game/Gameplay/Blueprints/Enemies/EnemySpawnManager.EnemySpawnManager_C|SetQuestCounter _returnvalue_2 (+ (Variables|/Game/Gameplay/Blueprints/Enemies/EnemySpawnManager.EnemySpawnManager_C|GetQuestCounter _returnvalue_2) 1))
            (Actor|DestroyActor)))))
    (:then_1
      ;[1 1 1] if attacking stop moving
      (if (or _returnvalue (Variables|Default|GetAttacking))
        (Components|Movement|StopMovementImmediately (Variables|Character|GetCharacterMovement))))
    (:then_2
      (CallFunction|Lockon))))

(fn ConstructionScript
  (bind _mesh (Variables|Character|GetMesh))
  (bind _returnvalue (Rendering|Material|CreateDynamicMaterialInstance "/Game/Gameplay/Materials/M_Range.M_Range" "None" "None" :!class /Script/Engine.KismetMaterialLibrary))
  (bind _output_get (Variables|Default|SetDMI_Range _returnvalue))
  (Rendering|Material|SetMaterial (Variables|Default|GetStaticMesh) 0 _output_get)
  (Components|SkeletalMesh|SetSkeletalMeshAsset _mesh (Variables|Default|GetEnemySkeletalMesh))
  (Class|SkeletalMeshComponent|SetAnimClass _mesh (Variables|Default|GetEnemyAnimBlueprint)))

(fn Lockon
  (bind _lockedonui (Variables|Default|GetLockedOnUI))
  (if (Variables|Default|GetLockedOn)
    (Rendering|SetVisibility _lockedonui true false)
    (else
      (Rendering|SetVisibility _lockedonui false false))))