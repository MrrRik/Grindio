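; Test lobbed projectile actor that moves toward a target location with a homing missile Niagara effect attached.
; BeginPlay starts a timeline whose Time output drives the blend alpha.
; Each Tick prints the target plus the timeline's curve offset and lerps from the current location toward it without sweep, so the start point shifts every frame.
; TargetLocation is not set within this Blueprint.
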(event EventBeginPlay
  (Components|Timeline|SetPlayRate (Variables|Default|GetTimeline) 1.0)
  (Niagara|SpawnSystemAttached "/Game/Gameplay/Effects/FX_HomingMissile.FX_HomingMissile" (Variables|Default|GetSphere1) "None" "0, 0, 0" "0, 0, 0" "KeepRelativeOffset" false)
  (bind (_direction _curve _time) (Timeline|Timeline PlayFromStart)
    (:Update
      (Variables|Default|SetCurve _time))))

(event EventTick
  (params (DeltaSeconds :type Float%20%28single-precision%29))
  (Development|PrintString (Utilities|String|ToString(Vector) (+ (Variables|Default|GetTargetLocation) (stale EventBeginPlay _curve))))
  (Transformation|SetActorLocation (Math|Vector|Lerp(Vector) (Transformation|GetActorLocation) (+ (Variables|Default|GetTargetLocation) (stale EventBeginPlay _curve)) (Math|Float|Clamp(Float) (Variables|Default|GetCurve))) false false))

(fn ConstructionScript)