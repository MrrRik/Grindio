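; Bullet is a projectile actor that damages a Hero, skeleton or spider on hit, briefly disabling its sphere collision at spawn.
; On hit it copies Damage from player 0's Hero, then calls GetHit on a struck Hero with a blood effect, or passes other actors to EnemyDamage.
; EnemyDamage matches exact skeleton or spider classes to apply damage and destroy the bullet; unmatched hits destroy it after a DamageInterval delay.
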(event OnComponentHit(Sphere1)
  (params (HitComponent :type Primitive%20Component%20Object%20Reference) (OtherActor :type Actor%20Object%20Reference) (OtherComp :type Primitive%20Component%20Object%20Reference) (NormalImpulse :type Vector :default "0, 0, 0") (Hit :type Hit%20Result%20Structure%20%28by%20ref%29))
  (bind _ashero (Utilities|Casting|CastToHero (Game|GetPlayerCharacter 0)))
  (Variables|Default|SetDamage (Variables|/Game/Gameplay/Blueprints/Hero/Hero.Hero_C|GetDamage _ashero))
  (Development|PrintString (Utilities|GetDisplayName OtherActor))
  (if (Utilities|ClassIsChildOf (Utilities|GetClass OtherActor) "/Game/Gameplay/Blueprints/Hero/Hero.Hero_C")
    (Utilities|FlowControl|DoOnce false
      (:Completed
        (bind _ashero_2 (Utilities|Casting|CastToHero OtherActor))
        (bind _output_get (Variables|/Game/Gameplay/Blueprints/Hero/Hero.Hero_C|SetGotHit _ashero_2 true))
        (Default|GetHit _ashero_2 (Variables|Default|GetDamage) _output_get)
        (Effects|SpawnEmitteratLocation "/Game/Packages/CartoonMeshParticles/Particles/Bloods/P_BloodExplosion_Short.P_BloodExplosion_Short" (.ImpactPoint (Collision|BreakHitResult Hit)) "0, 0, 0" "1.000000,1.000000,1.000000" true "AutoRelease")))
    (else
      (CallFunction|EnemyDamage OtherActor)
      (Utilities|FlowControl|Delay (Variables|Default|GetDamageInterval))))
  (Actor|DestroyActor))

(event EventBeginPlay
  (bind _sphere1 (Variables|Default|GetSphere1))
  (Collision|SetCollisionEnabled _sphere1 "NoCollision")
  (Utilities|FlowControl|Delay 0.01)
  (Collision|SetCollisionEnabled _sphere1 "QueryAndPhysics"))

(fn ConstructionScript)

(fn EnemyDamage
  (params (EnemyActor :type Actor%20Object%20Reference))
  (bind _returnvalue (Utilities|GetClass EnemyActor))
  (bind _damage (Variables|Default|GetDamage))
  (Utilities|FlowControl|DoOnce false
    (:Completed
      (if (== _returnvalue "/Game/Gameplay/Blueprints/Enemies/Enemy_Skeleton.Enemy_Skeleton_C")
        (bind _asenemy_skeleton (Utilities|Casting|CastToEnemy_Skeleton EnemyActor))
        (bind _output_get (Variables|/Game/Gameplay/Blueprints/Enemies/Enemy_Skeleton.Enemy_Skeleton_C|SetGotHit _asenemy_skeleton true))
        (Default|GetHit _asenemy_skeleton _output_get _damage)
        (Actor|DestroyActor)
        (else
          (Development|PrintString "Hit is not skeleton")
          (if (== _returnvalue "/Game/Gameplay/Blueprints/Enemies/Enemy_Spider.Enemy_Spider_C")
            (bind _asenemy_spider (Utilities|Casting|CastToEnemy_Spider EnemyActor))
            (bind _output_get_2 (Variables|/Game/Gameplay/Blueprints/Enemies/Enemy_Spider.Enemy_Spider_C|SetGotHit _asenemy_spider true))
            (Default|GetHit _asenemy_spider _output_get_2 _damage)
            (Actor|DestroyActor)
            (else
              (Development|PrintString "hit is not spider"))))))))