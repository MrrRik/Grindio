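; Base Blueprint for a hero part that displays one skeletal mesh, chosen from PartMesh by the SkeletalMesh variable.
; The Construction Script applies the selected mesh to PartComponent.
; BeginPlay applies the mesh again and sets the component's animation class from AnimClass.
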(event EventBeginPlay
  ;[0 0 0] Set which skeletal mesh to use
  (Components|SkeletalMesh|SetSkeletalMeshAsset (Variables|Default|GetPartComponent) (Utilities|Array|Get(acopy) (Variables|Default|GetPartMesh) (Variables|Default|GetSkeletalMesh)))
  (Class|SkeletalMeshComponent|SetAnimClass (Variables|Default|GetPartComponent) (Variables|Default|GetAnimClass)))

(fn ConstructionScript
  (Components|SkeletalMesh|SetSkeletalMeshAsset (Variables|Default|GetPartComponent) (Utilities|Array|Get(acopy) (Variables|Default|GetPartMesh) (Variables|Default|GetSkeletalMesh))))