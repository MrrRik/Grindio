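; Hero sword Blueprint that deals the player's damage to skeleton and spider enemies it hits.
; A Box hit reads Damage from the player's 0_Hero_J, prints the struck actor's name and sends non-hero actors to EnemyDamage.
; EnemyDamage matches exact enemy classes, then sets GotHit and calls GetHit, behind a DoOnce with no visible reset.
; Hero-damage, blood-effect and collision-toggle logic is left disconnected.
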(event OnComponentHit(Box)
  (params (HitComponent :type Primitive%20Component%20Object%20Reference) (OtherActor :type Actor%20Object%20Reference) (OtherComp :type Primitive%20Component%20Object%20Reference) (NormalImpulse :type Vector :default "0, 0, 0") (Hit :type Hit%20Result%20Structure%20%28by%20ref%29))
  (bind _as0_hero_j (Utilities|Casting|CastTo0_Hero_J (Game|GetPlayerCharacter 0)))
  (Variables|Default|SetDamage (Variables|/Game/Gameplay/Blueprints/Hero/0_Hero_J.0_Hero_J_C|GetDamage _as0_hero_j))
  (Development|PrintString (Utilities|GetDisplayName OtherActor))
  (if (not (Utilities|ClassIsChildOf (Utilities|GetClass OtherActor) "/Game/Gameplay/Blueprints/Hero/0_Hero_J.0_Hero_J_C"))
    (CallFunction|EnemyDamage OtherActor)))

(event EventBeginPlay)

(fn ConstructionScript)

(fn EnemyDamage
  (params (EnemyActor :type Actor%20Object%20Reference))
  (bind _returnvalue (Utilities|GetClass EnemyActor))
  (bind _damage (Variables|Default|GetDamage))
  (Utilities|FlowControl|DoOnce false
    (:Completed
      (if (== _returnvalue "/Game/Gameplay/Blueprints/Enemies/Enemy_Skeleton.Enemy_Skeleton_C")
        (bind _asenemy_skeleton (Utilities|Casting|CastToEnemy_Skeleton EnemyActor))
        (bind _output_get (Variables|/Game/Gameplay/Blueprints/Enemies/Enemy_Skeleton.Enemy_Skeleton_C|SetGotHit _asenemy_skeleton true))
        (Default|GetHit _asenemy_skeleton _output_get _damage)
        (else
          (Development|PrintString "Hit is not skeleton")
          (if (== _returnvalue "/Game/Gameplay/Blueprints/Enemies/Enemy_Spider.Enemy_Spider_C")
            (bind _asenemy_spider (Utilities|Casting|CastToEnemy_Spider EnemyActor))
            (bind _output_get_2 (Variables|/Game/Gameplay/Blueprints/Enemies/Enemy_Spider.Enemy_Spider_C|SetGotHit _asenemy_spider true))
            (Default|GetHit _asenemy_spider _output_get_2 _damage)
            (else
              (Development|PrintString "hit is not spider"))))))))