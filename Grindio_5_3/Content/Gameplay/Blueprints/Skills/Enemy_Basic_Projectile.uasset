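; Basic enemy projectile that damages the Hero on hit and destroys itself on any impact.
; BeginPlay derives the movement component's initial speed from BulletSpeed and keeps the sphere's collision off for a brief delay before enabling it.
; The sphere's hit event calls the Hero's damage function with the projectile's Damage.
; A separate EnemyDamage graph, not called here, applies one-time damage to Enemy_Base actors.
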(event OnComponentHit(Sphere1)
  (params (HitComponent :type Primitive%20Component%20Object%20Reference) (OtherActor :type Actor%20Object%20Reference) (OtherComp :type Primitive%20Component%20Object%20Reference) (NormalImpulse :type Vector :default "0, 0, 0") (Hit :type Hit%20Result%20Structure%20%28by%20ref%29))
  (if (Utilities|ClassIsChildOf (Utilities|GetClass OtherActor) "/Game/Gameplay/Blueprints/Hero/Hero.Hero_C")
    (bind _ashero (Utilities|Casting|CastToHero OtherActor))
    (Default|HeroIsDealtDamage _ashero true (Variables|Default|GetDamage))
    (Actor|DestroyActor)
    (else
      (Actor|DestroyActor))))

(event EventBeginPlay
  (bind _sphere1 (Variables|Default|GetSphere1))
  (Variables|/Script/Engine.ProjectileMovementComponent|SetInitialSpeed (Variables|Default|GetProjectileMovement) (* (Variables|Default|GetBulletSpeed) 5e+03))
  (Collision|SetCollisionEnabled _sphere1 "NoCollision")
  (Utilities|FlowControl|Delay 0.1)
  (Collision|SetCollisionEnabled _sphere1 "QueryAndPhysics"))

(fn ConstructionScript)

(fn EnemyDamage
  (params (EnemyActor :type Actor%20Object%20Reference))
  (Utilities|FlowControl|DoOnce false
    (:Completed
      (if (Utilities|ClassIsChildOf (Utilities|GetClass EnemyActor) "/Game/Gameplay/Blueprints/Enemies/Enemy_Base.Enemy_Base_C")
        (bind _asenemy_base (Utilities|Casting|CastToEnemy_Base EnemyActor))
        (bind _output_get (Variables|/Game/Gameplay/Blueprints/Enemies/Enemy_Base.Enemy_Base_C|SetGotHit _asenemy_base true))
        (Default|EnemyIsDealtDamage _asenemy_base _output_get (Variables|Default|GetDamage))
        (Actor|DestroyActor)))))