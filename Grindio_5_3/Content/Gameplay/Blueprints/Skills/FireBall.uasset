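; FireBall skill actor that deals damage on sphere hit, using the Damage value read from the player's Hero.
; A hit Hero is flagged, receives GetHit and spawns a blood explosion before the fireball is destroyed.
; Other actors go through EnemyDamage, which damages only exact Enemy_Base instances, with delayed destruction as fallback.
; DoOnce gates limit each damage path to a single application.
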(event OnComponentBeginOverlap(Sphere1)
  (params (OverlappedComponent :type Primitive%20Component%20Object%20Reference) (OtherActor :type Actor%20Object%20Reference) (OtherComp :type Primitive%20Component%20Object%20Reference) (OtherBodyIndex :type Integer) (bFromSweep :type Boolean) (SweepResult :type Hit%20Result%20Structure%20%28by%20ref%29)))

(event OnComponentHit(Sphere1)
  (params (HitComponent :type Primitive%20Component%20Object%20Reference) (OtherActor :type Actor%20Object%20Reference) (OtherComp :type Primitive%20Component%20Object%20Reference) (NormalImpulse :type Vector :default "0, 0, 0") (Hit :type Hit%20Result%20Structure%20%28by%20ref%29))
  (bind _ashero (Utilities|Casting|CastToHero (Game|GetPlayerCharacter 0)))
  (Variables|Default|SetDamage (Variables|/Game/Gameplay/Blueprints/Hero/Hero.Hero_C|GetDamage _ashero))
  (Development|PrintString (Utilities|GetDisplayName OtherActor))
  (if (Utilities|ClassIsChildOf (Utilities|GetClass OtherActor) "/Game/Gameplay/Blueprints/Hero/Hero.Hero_C")
    (Utilities|FlowControl|DoOnce false
      (:Completed
        (bind _ashero_2 (Utilities|Casting|CastToHero OtherActor))
        (bind _output_get (Variables|/Game/Gameplay/Blueprints/Hero/Hero.Hero_C|SetGotHit _ashero_2 true))
        (Default|GetHit _ashero_2 (Variables|Default|GetDamage) _output_get)
        (Effects|SpawnEmitteratLocation "/Game/Packages/CartoonMeshParticles/Particles/Bloods/P_BloodExplosion_Short.P_BloodExplosion_Short" (.ImpactPoint (Collision|BreakHitResult Hit)) "0, 0, 0" "1.000000,1.000000,1.000000" true "AutoRelease")))
    (else
      (CallFunction|EnemyDamage OtherActor)
      (Utilities|FlowControl|Delay (Variables|Default|GetDamageInterval))))
  (Actor|DestroyActor))

(fn ConstructionScript)

(fn EnemyDamage
  (params (EnemyActor :type Actor%20Object%20Reference))
  (Utilities|FlowControl|DoOnce false
    (:Completed
      (if (== (Utilities|GetClass EnemyActor) "/Game/Gameplay/Blueprints/Enemies/Enemy_Base.Enemy_Base_C")
        (bind _asenemy_base (Utilities|Casting|CastToEnemy_Base EnemyActor))
        (bind _output_get (Variables|/Game/Gameplay/Blueprints/Enemies/Enemy_Base.Enemy_Base_C|SetGotHit _asenemy_base true))
        (Default|GetHit _asenemy_base _output_get (Variables|Default|GetDamage))
        (Actor|DestroyActor)))))