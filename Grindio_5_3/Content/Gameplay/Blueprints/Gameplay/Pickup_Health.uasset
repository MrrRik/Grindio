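; Health pickup that restores a Hero's health by HealthBoost, capped at MaxHealth.
; Any overlap with its sphere swaps the loot particle for a health-increase effect and plays a 2D sound.
; Healing waits until that effect finishes, casting the overlapped actor to Hero at that point.
; The pickup then destroys itself, even if the Hero was at full health, but stays if the cast fails.
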(event OnComponentBeginOverlap(Sphere)
  (params (OverlappedComponent :type Primitive%20Component%20Object%20Reference) (OtherActor :type Actor%20Object%20Reference) (OtherComp :type Primitive%20Component%20Object%20Reference) (OtherBodyIndex :type Integer) (bFromSweep :type Boolean) (SweepResult :type Hit%20Result%20Structure%20%28by%20ref%29))
  (Components|Activation|Deactivate (Variables|Default|GetP_Loot_Red))
  (Components|Activation|Activate (Variables|Default|GetP_HealthIncrease) false)
  (Audio|PlaySound2D "/Game/Packages/Interface_And_Item_Sounds/Cues/Special_Powerup_03_Cue.Special_Powerup_03_Cue" 1.0 1.0 0.0 0 0))

(event OnSystemFinished(P_HealthIncrease)
  (params (PSystem :type Particle%20System%20Component%20Object%20Reference))
  (bind _ashero (Utilities|Casting|CastToHero (stale OnComponentBeginOverlap(Sphere) OtherActor)))
  ;[1 1 1] check if hero is not already full hp
  (if (< (Variables|/Game/Gameplay/Blueprints/Hero/Hero.Hero_C|GetCurrentHealth _ashero) (Variables|/Game/Gameplay/Blueprints/Hero/Hero.Hero_C|GetMaxHealth _ashero))
    ;[1 1 1] check if hero doesnt go over max hp by healing (if so new hp is max hp)
    (if (> (+ (Variables|/Game/Gameplay/Blueprints/Hero/Hero.Hero_C|GetCurrentHealth _ashero) (Variables|Default|GetHealthBoost)) (Variables|/Game/Gameplay/Blueprints/Hero/Hero.Hero_C|GetMaxHealth _ashero))
      (Variables|/Game/Gameplay/Blueprints/Hero/Hero.Hero_C|SetCurrentHealth _ashero (Variables|/Game/Gameplay/Blueprints/Hero/Hero.Hero_C|GetMaxHealth _ashero))
      (else
        (Variables|/Game/Gameplay/Blueprints/Hero/Hero.Hero_C|SetCurrentHealth _ashero (+ (Variables|/Game/Gameplay/Blueprints/Hero/Hero.Hero_C|GetCurrentHealth _ashero) (Variables|Default|GetHealthBoost))))))
  (Actor|DestroyActor))

(fn ConstructionScript)