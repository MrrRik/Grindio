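; Coin pickup actor that plays a sound on spawn and adds its value to the Hero's coin count when collected.
; Overlapping its sphere disables collision and starts a timeline that pulls the coin toward a point below the overlapping actor, switching off the loot particle shortly after.
; When the timeline finishes, a Hero cast gates the reward, pickup sound and increase particle, whose completion destroys the actor.
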(event OnComponentBeginOverlap(Sphere)
  (params (OverlappedComponent :type Primitive%20Component%20Object%20Reference) (OtherActor :type Actor%20Object%20Reference) (OtherComp :type Primitive%20Component%20Object%20Reference) (OtherBodyIndex :type Integer) (bFromSweep :type Boolean) (SweepResult :type Hit%20Result%20Structure%20%28by%20ref%29))
  (Collision|SetActorEnableCollision false)
  (bind _alpha (Timeline|Timeline_0 PlayFromStart)
    (:Update
      (Transformation|SetActorLocation (Math|Vector|Lerp(Vector) (Transformation|GetActorLocation self) (- (Transformation|GetWorldLocation (Variables|/Script/Engine.Actor|GetRootComponent OtherActor)) "0.000000,0.000000,50.000000") _alpha) false false)
      (if (>= _alpha 0.1)
        (Components|Activation|Deactivate (Variables|Default|GetP_Loot_Yellow))))
    (:Finished
      (bind _ashero (Utilities|Casting|CastToHero OtherActor))
      (Variables|/Game/Gameplay/Blueprints/Hero/Hero.Hero_C|SetCoin _ashero (+ (Variables|/Game/Gameplay/Blueprints/Hero/Hero.Hero_C|GetCoin _ashero) (Variables|Default|GetCoinValue)))
      (Components|Activation|Activate (Variables|Default|GetP_CoinIncrease) false)
      (Audio|PlaySound2D "/Game/Packages/Interface_And_Item_Sounds/Cues/Item_Sell_Purchase_03_Cue.Item_Sell_Purchase_03_Cue" 1.0 1.0 0.0 0 0))))

(event OnSystemFinished(P_CoinIncrease)
  (params (PSystem :type Particle%20System%20Component%20Object%20Reference))
  (Actor|DestroyActor))

(event EventBeginPlay
  (Audio|PlaySound2D "/Game/Packages/Interface_And_Item_Sounds/Cues/Coins_08_Cue.Coins_08_Cue" 1.0 1.0 0.0 0 0))

(fn ConstructionScript)