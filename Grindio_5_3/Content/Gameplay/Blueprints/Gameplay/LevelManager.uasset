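; LevelManager is a level-exit trigger that advances the game to the next numbered level when its Box begins an overlap, with no check on the overlapping actor.
; The overlap plays the FadeToBlack level sequence, waits briefly, then opens the next level by name.
; That name is derived by splitting the current level name at the underscore and incrementing the number, with a hard-coded leading zero that assumes single-digit numbering.
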(event OnComponentBeginOverlap(Box)
  (params (OverlappedComponent :type Primitive%20Component%20Object%20Reference) (OtherActor :type Actor%20Object%20Reference) (OtherComp :type Primitive%20Component%20Object%20Reference) (OtherBodyIndex :type Integer) (bFromSweep :type Boolean) (SweepResult :type Hit%20Result%20Structure%20%28by%20ref%29))
  (bind _returnvalue (Game|GetCurrentLevelName true))
  (bind _outactor (Sequencer|Player|CreateLevelSequencePlayer "/Game/Gameplay/Sequences/FadeToBlack.FadeToBlack"))
  (Sequencer|Player|Play (Variables|/Script/LevelSequence.LevelSequenceActor|GetSequencePlayer _outactor) :!class /Script/MovieScene.MovieSceneSequencePlayer)
  (Utilities|FlowControl|Delay 1.0)
  (Game|OpenLevel(byName) (Utilities|String|StringToName (Utilities|String|Append (.LeftS (Utilities|String|Split _returnvalue "_" "CaseSensitive")) "_0" (Utilities|String|ToString(Integer) (+ (.RightS (Utilities|String|Split _returnvalue "_" "CaseSensitive")) 1))))))

(fn ConstructionScript)