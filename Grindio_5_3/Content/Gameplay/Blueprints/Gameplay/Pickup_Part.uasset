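; Body-part pickup that flies into the player's Hero and swaps in a dropped helmet, arm or legs part.
; Sphere overlap disables collision and runs a timeline that lerps the pickup toward the overlapping actor while shutting off its Niagara effect.
; On finish, Spawn flags select indexed parts for the Hero, with right and left arm flags crossed.
; Coin effect and sound accompany pickup; the actor self-destroys when the effect finishes.
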(event OnComponentBeginOverlap(Sphere)
  (params (OverlappedComponent :type Primitive%20Component%20Object%20Reference) (OtherActor :type Actor%20Object%20Reference) (OtherComp :type Primitive%20Component%20Object%20Reference) (OtherBodyIndex :type Integer) (bFromSweep :type Boolean) (SweepResult :type Hit%20Result%20Structure%20%28by%20ref%29))
  (Collision|SetActorEnableCollision false)
  (bind _alpha (Timeline|Timeline_0 PlayFromStart)
    (:Update
      (Transformation|SetActorLocation (Math|Vector|Lerp(Vector) (Transformation|GetActorLocation self) (- (Transformation|GetWorldLocation (Variables|/Script/Engine.Actor|GetRootComponent OtherActor)) "0.000000,0.000000,50.000000") _alpha) false false)
      (if (>= _alpha 0.1)
        (Components|Activation|Deactivate (Variables|Default|GetNiagara))))
    (:Finished
      (bind _ashero (Utilities|Casting|CastToHero OtherActor))
      (Utilities|FlowControl|Sequence
        (:then_0
          (if (Variables|Default|GetSpawnHelmet)
            (Default|PartHelmUpdate _ashero (Utilities|Array|Get(acopy) (Variables|Default|GetHelmets) (Variables|Default|GetDroppedHelmetIndex)))
            (Components|Activation|Activate (Variables|Default|GetP_CoinIncrease) false :!label _label)
            (Audio|PlaySound2D "/Game/Packages/Interface_And_Item_Sounds/Cues/Item_Sell_Purchase_03_Cue.Item_Sell_Purchase_03_Cue" 1.0 1.0 0.0 0 0)
            (else
              (if (Variables|Default|GetSpawnRArm) :!label _label_2
                (Default|PartLArmUpdate _ashero (Utilities|Array|Get(acopy) (Variables|Default|GetLArms) (Variables|Default|GetDroppedLArmIndex)))
                (goto _label)
                (else
                  (if (Variables|Default|GetSpawnLArm) :!label _label_3
                    (Default|PartRArmUpdate _ashero (Utilities|Array|Get(acopy) (Variables|Default|GetRArms) (Variables|Default|GetDroppedRArmIndex)))
                    (goto _label)
                    (else
                      (if (Variables|Default|GetSpawnLegs) :!label _label_4
                        (Default|PartLegsUpdate _ashero (Utilities|Array|Get(acopy) (Variables|Default|GetLegs) (Variables|Default|GetDroppedLegsIndex)))
                        (goto _label)))))))))
        (:then_1
          (goto _label_2))
        (:then_2
          (goto _label_3))
        (:then_3
          (goto _label_4))))))

(event OnSystemFinished(P_CoinIncrease)
  (params (PSystem :type Particle%20System%20Component%20Object%20Reference))
  (Actor|DestroyActor))

(event EventBeginPlay
  (Audio|PlaySound2D "/Game/Packages/Interface_And_Item_Sounds/Cues/Coins_08_Cue.Coins_08_Cue" 1.0 1.0 0.0 0 0))

(fn ConstructionScript
  (Utilities|FlowControl|Sequence
    (:then_0
      (if (Variables|Default|GetSpawnHelmet)
        _))
    (:then_1
      (if (Variables|Default|GetSpawnRArm)
        _))
    (:then_2
      (if (Variables|Default|GetSpawnLArm)
        _))
    (:then_3
      (if (Variables|Default|GetSpawnLegs)
        _))))