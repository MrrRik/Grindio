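; Enemy character that roams the navmesh, chases the Hero on entering its far collision and flags attacking within the near one, recolouring its range material per state.
; A ball collider on a mesh socket flags hits and passes damage to the Hero.
; Tick feeds the health widget, halts movement while attacking or dead, and triggers death once.
; Death fires a coin-spray particle whose collisions spawn coins or occasional health pickups, then smoke, then destruction.
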(event OnComponentBeginOverlap(ballCollision)
  (params (OverlappedComponent :type Primitive%20Component%20Object%20Reference) (OtherActor :type Actor%20Object%20Reference) (OtherComp :type Primitive%20Component%20Object%20Reference) (OtherBodyIndex :type Integer) (bFromSweep :type Boolean) (SweepResult :type Hit%20Result%20Structure%20%28by%20ref%29))
  ;[1 1 1] Hit hero detection
  (if (== (Utilities|GetClass OtherActor) "/Game/Gameplay/Blueprints/Hero.Hero_C")
    (bind _ashero (Utilities|Casting|CastToHero (Game|Player|GetPlayerPawn 0)))
    (Variables|/Game/Gameplay/Blueprints/Hero.Hero_C|SetGotHit _ashero true)
    (Variables|/Game/Gameplay/Blueprints/Hero.Hero_C|SetDamage _ashero (Variables|Default|GetEnemyDefaultDamage))))

(event OnParticleCollide(PS_CoinSpray)
  (params (EventName :type Name :default "None") (EmitterTime :type Float%20%28single-precision%29) (ParticleTime :type Integer) (Location :type Vector :default "0, 0, 0") (Velocity :type Vector :default "0, 0, 0") (Direction :type Vector :default "0, 0, 0") (Normal :type Vector :default "0, 0, 0") (BoneName :type Name :default "None") (PhysMat :type Physical%20Material%20Object%20Reference))
  (bind _returnvalue (+ Location "0, 0,40.000000"))
  (bind _returnvalue_2 (Math|Conversions|ToTransform(Vector) _returnvalue))
  (if (> (Math|Random|RandomIntegerinRange 0 10) 9)
    (Game|SpawnActorfromClass "/Game/Gameplay/Blueprints/Health.Health_C" _returnvalue_2 "AlwaysSpawn" 0 0)
    (else
      (Game|SpawnActorfromClass "/Game/Gameplay/Blueprints/Coin.Coin_C" _returnvalue_2 "AlwaysSpawn" 0 0))))

(event OnComponentBeginOverlap(nearbyCol)
  (params (OverlappedComponent :type Primitive%20Component%20Object%20Reference) (OtherActor :type Actor%20Object%20Reference) (OtherComp :type Primitive%20Component%20Object%20Reference) (OtherBodyIndex :type Integer) (bFromSweep :type Boolean) (SweepResult :type Hit%20Result%20Structure%20%28by%20ref%29))
  ;[1 1 1] If close hero detection
  (if (== (Utilities|GetClass OtherActor) "/Game/Gameplay/Blueprints/Hero.Hero_C")
    (Variables|Default|SetAttacking true)
    (Rendering|Material|SetVectorParameterValue (Variables|Default|GetDMI_Range) "Color" "(R=1.000000,G=0.000000,B=0.000000,A=1.000000)" :!class /Script/Engine.MaterialInstanceDynamic)))

(event OnComponentEndOverlap(nearbyCol)
  (params (OverlappedComponent :type Primitive%20Component%20Object%20Reference) (OtherActor :type Actor%20Object%20Reference) (OtherComp :type Primitive%20Component%20Object%20Reference) (OtherBodyIndex :type Integer))
  ;[1 1 1] If close hero detection
  (if (== (Utilities|GetClass OtherActor) "/Game/Gameplay/Blueprints/Hero.Hero_C")
    (Utilities|FlowControl|Delay 2.6)
    (Variables|Default|SetAttacking false)
    (CallFunction|ChasePlayer)))

(event OnComponentBeginOverlap(FarCol)
  (params (OverlappedComponent :type Primitive%20Component%20Object%20Reference) (OtherActor :type Actor%20Object%20Reference) (OtherComp :type Primitive%20Component%20Object%20Reference) (OtherBodyIndex :type Integer) (bFromSweep :type Boolean) (SweepResult :type Hit%20Result%20Structure%20%28by%20ref%29))
  ;[1 1 1] Far away hero detection
  (if (== (Utilities|GetClass OtherActor) "/Game/Gameplay/Blueprints/Hero.Hero_C")
    (CallFunction|ChasePlayer)))

(event OnComponentEndOverlap(FarCol)
  (params (OverlappedComponent :type Primitive%20Component%20Object%20Reference) (OtherActor :type Actor%20Object%20Reference) (OtherComp :type Primitive%20Component%20Object%20Reference) (OtherBodyIndex :type Integer))
  ;[1 1 1] Far away hero detection
  (if (== (Utilities|GetClass OtherActor) "/Game/Gameplay/Blueprints/Hero.Hero_C")
    (CallFunction|Roam)))

(event Custom|Roam
  ;[1 1 1] Roaming event
  (Rendering|Material|SetVectorParameterValue (Variables|Default|GetDMI_Range) "Color" "(R=0.000000,G=0.897796,B=1.000000,A=1.000000)" :!class /Script/Engine.MaterialInstanceDynamic)
  (AI|AIMoveTo self (.RandomLocation (Class|NavigationSystemV1|GetRandomPointinNavigableRadius (Transformation|GetActorLocation) (Variables|Default|Getradius) 0 0)) 0 5.0 false
    (:OnSuccess
      (Utilities|FlowControl|Delay 1.0)
      (CallFunction|Roam))))

(event Custom|ChasePlayer
  ;[1 1 1] Chasing player event
  (Rendering|Material|SetVectorParameterValue (Variables|Default|GetDMI_Range) "Color" "(R=1.000000,G=0.341622,B=0.000000,A=1.000000)" :!class /Script/Engine.MaterialInstanceDynamic)
  (AI|AIMoveTo self "0, 0, 0" (Game|GetPlayerCharacter 0) 1.5e+02 false
    (:OnSuccess
      (Utilities|FlowControl|Delay 1.0)
      (CallFunction|ChasePlayer))))

(event EventBeginPlay
  ;[1 1 1] Set max hp and start roaming
  (Utilities|FlowControl|Sequence
    (:then_0
      (CallFunction|Roam))
    (:then_1
      (Variables|Default|SetCurrentHealth (Variables|Default|GetMaxHealth))
      (bind _asenemy_hud (Utilities|Casting|CastToEnemy_HUD (UserInterface|GetUserWidgetObject (Variables|Default|GetEnemyHealthUI))))
      (Variables|/Game/Gameplay/UI/Enemy_HUD.Enemy_HUD_C|SetMaxHealth_UI _asenemy_hud (Variables|Default|GetMaxHealth)))))

(event EventTick
  (params (DeltaSeconds :type Float%20%28single-precision%29))
  (bind _currenthealth (Variables|Default|GetCurrentHealth))
  (bind _returnvalue (<= _currenthealth 0.0))
  (Utilities|FlowControl|Sequence
    (:then_0
      ;[1 1 1] Dying
      (if _returnvalue
        (Utilities|FlowControl|DoOnce false
          (:Completed
            (Components|Activation|Activate (Variables|Default|GetPS_CoinSpray) false)
            (Utilities|FlowControl|Delay 0.3)
            (Effects|SpawnEmitteratLocation "/Game/Gameplay/Effects/PS_Smoke.PS_Smoke" (- (Transformation|GetWorldLocation (Variables|Default|GetStaticMesh1)) "0, 0,-6.500000"))
            (Utilities|FlowControl|Delay 0.7)
            (Actor|DestroyActor)))))
    (:then_1
      ;[1 1 1] if attacking stop moving
      (if (or (Variables|Default|GetAttacking) _returnvalue)
        (Components|Movement|StopMovementImmediately (Variables|Character|GetCharacterMovement))))
    (:then_2
      ;[1 1 1] setting healthbar
      (bind _asenemy_hud (Utilities|Casting|CastToEnemy_HUD (UserInterface|GetUserWidgetObject (Variables|Default|GetEnemyHealthUI))))
      (Variables|/Game/Gameplay/UI/Enemy_HUD.Enemy_HUD_C|SetCurrentHealth_UI _asenemy_hud (Variables|Default|GetCurrentHealth)))))

(fn ConstructionScript
  (Transformation|AttachComponentToComponent (Variables|Default|GetballCollision) (Variables|Character|GetMesh) "ballSocket" "KeepRelative" "KeepRelative" "KeepRelative" true)
  (bind _returnvalue (Rendering|Material|CreateDynamicMaterialInstance "/Game/Gameplay/Materials/M_Range.M_Range" "None" :!class /Script/Engine.KismetMaterialLibrary))
  (bind _output_get (Variables|Default|SetDMI_Range _returnvalue))
  (Rendering|Material|SetMaterial (Variables|Default|GetStaticMesh) 0 _output_get))