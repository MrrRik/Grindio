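; Health pickup that restores hero health by a boost amount, capped at the maximum.
; Any overlap with its sphere switches off the red loot particle and plays the health increase effect.
; When that effect finishes, it casts the overlapping actor to the hero, applies the heal if health is below maximum, and destroys itself.
; If the cast fails, the pickup is neither applied nor destroyed.
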(event OnComponentBeginOverlap(Sphere)
  (params (OverlappedComponent :type Primitive%20Component%20Object%20Reference) (OtherActor :type Actor%20Object%20Reference) (OtherComp :type Primitive%20Component%20Object%20Reference) (OtherBodyIndex :type Integer) (bFromSweep :type Boolean) (SweepResult :type Hit%20Result%20Structure%20%28by%20ref%29))
  (Components|Activation|Deactivate (Variables|Default|GetP_Loot_Red))
  (Components|Activation|Activate (Variables|Default|GetP_HealthIncrease) false))

(event OnSystemFinished(P_HealthIncrease)
  (params (PSystem :type Particle%20System%20Component%20Object%20Reference))
  (bind _as0_hero (Utilities|Casting|CastTo0_Hero (stale OnComponentBeginOverlap(Sphere) OtherActor)))
  ;[1 1 1] check if hero is not already full hp
  (if (< (Variables|/Game/Gameplay/Blueprints/Hero/0_Hero.0_Hero_C|GetCurrentHealth _as0_hero) (Variables|/Game/Gameplay/Blueprints/Hero/0_Hero.0_Hero_C|GetMaxHealth _as0_hero))
    ;[1 1 1] check if hero doesnt go over max hp by healing (if so new hp is max hp)
    (if (> (+ (Variables|/Game/Gameplay/Blueprints/Hero/0_Hero.0_Hero_C|GetCurrentHealth _as0_hero) (Variables|Default|GetHealthBoost)) (Variables|/Game/Gameplay/Blueprints/Hero/0_Hero.0_Hero_C|GetMaxHealth _as0_hero))
      (Variables|/Game/Gameplay/Blueprints/Hero/0_Hero.0_Hero_C|SetCurrentHealth _as0_hero (Variables|/Game/Gameplay/Blueprints/Hero/0_Hero.0_Hero_C|GetMaxHealth _as0_hero))
      (else
        (Variables|/Game/Gameplay/Blueprints/Hero/0_Hero.0_Hero_C|SetCurrentHealth _as0_hero (+ (Variables|/Game/Gameplay/Blueprints/Hero/0_Hero.0_Hero_C|GetCurrentHealth _as0_hero) (Variables|Default|GetHealthBoost))))))
  (Actor|DestroyActor))

(event EventBeginPlay)

(event Collision|EventActorBeginOverlap
  (params (OtherActor :type Actor%20Object%20Reference)))

(event EventTick
  (params (DeltaSeconds :type Float%20%28single-precision%29)))

(fn ConstructionScript)