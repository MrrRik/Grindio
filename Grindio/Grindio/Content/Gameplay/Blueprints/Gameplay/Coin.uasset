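; Coin pickup actor that flies to the hero on overlap and adds its value to the hero's coin count.
; Overlap with the hero disables the coin's collision and plays a timeline that lerps it toward the hero's mesh, switching off the yellow loot effect early in the motion.
; When the timeline finishes, the coin value is added and a coin-increase particle effect plays, whose completion destroys the actor.
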(event OnComponentBeginOverlap(Sphere)
  (params (OverlappedComponent :type Primitive%20Component%20Object%20Reference) (OtherActor :type Actor%20Object%20Reference) (OtherComp :type Primitive%20Component%20Object%20Reference) (OtherBodyIndex :type Integer) (bFromSweep :type Boolean) (SweepResult :type Hit%20Result%20Structure%20%28by%20ref%29))
  (bind _as0_hero (Utilities|Casting|CastTo0_Hero OtherActor))
  (Collision|SetActorEnableCollision false)
  (bind _alpha (Timeline|Timeline_0 PlayFromStart)
    (:Update
      (Transformation|SetActorLocation (Math|Vector|Lerp(Vector) (Transformation|GetActorLocation self) (Transformation|GetWorldLocation (Variables|/Script/Engine.Character|GetMesh _as0_hero)) _alpha) false false)
      (if (>= _alpha 0.1)
        (Components|Activation|Deactivate (Variables|Default|GetP_Loot_Yellow))))
    (:Finished
      (bind _as0_hero_2 (Utilities|Casting|CastTo0_Hero OtherActor))
      (Variables|/Game/Gameplay/Blueprints/Hero/0_Hero.0_Hero_C|SetCoin _as0_hero_2 (+ (Variables|/Game/Gameplay/Blueprints/Hero/0_Hero.0_Hero_C|GetCoin _as0_hero_2) (Variables|Default|GetCoinValue)))
      (Components|Activation|Activate (Variables|Default|GetP_CoinIncrease) false))))

(event OnSystemFinished(P_CoinIncrease)
  (params (PSystem :type Particle%20System%20Component%20Object%20Reference))
  (Actor|DestroyActor))

(event EventTick
  (params (DeltaSeconds :type Float%20%28single-precision%29)))

(fn ConstructionScript)