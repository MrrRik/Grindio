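; Main menu game mode that dresses the hero character in the player's saved armor set.
; On BeginPlay it finds the 0_Hero actor, loads the PlayerSettingsSave slot and passes the stored player info into the hero's fixed outfit indexes before rebuilding the outfit.
; If no save exists, it creates and saves one from its own PlayerInfo, leaving the hero's outfit untouched.
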(event Custom|UpdateMainMenuCharacter
  ;[1 1 1] Updates the main menu character with the saved armor set the player picked
  (bind _returnvalue (Actor|GetActorOfClass "/Game/Gameplay/Blueprints/0_Hero.0_Hero_C"))
  (bind _output_get (Variables|Default|SetHeroRef _returnvalue))
  (bind _returnvalue_2 (SaveGame|DoesSaveGameExist (Variables|Default|GetPlayerSettingsSave)))
  (if _returnvalue_2
    (bind _returnvalue_3 (SaveGame|LoadGamefromSlot (Variables|Default|GetPlayerSettingsSave)))
    (bind _asplayer_save_game (Utilities|Casting|CastToPlayerSaveGame _returnvalue_3))
    (Default|SetFixedOutfitIndexes _output_get (Variables|/Game/Gameplay/Blueprints/PlayerSaveGame.PlayerSaveGame_C|GetS_PlayerInfo _asplayer_save_game))
    (Default|FMakeOutfit _output_get)
    (else
      (bind _returnvalue_4 (SaveGame|CreateSaveGameObject "/Game/Gameplay/Blueprints/PlayerSaveGame.PlayerSaveGame_C"))
      (Variables|Default|SetSaveGameRef _returnvalue_4)
      (Variables|/Game/Gameplay/Blueprints/PlayerSaveGame.PlayerSaveGame_C|SetS_PlayerInfo (Variables|Default|GetSaveGameRef) (Variables|Default|GetPlayerInfo))
      (SaveGame|SaveGametoSlot (Variables|Default|GetSaveGameRef) (Variables|Default|GetPlayerSettingsSave)))))

(event EventBeginPlay
  (CallFunction|UpdateMainMenuCharacter))

(fn ConstructionScript)