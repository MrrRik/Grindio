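; Bullet projectile actor that damages Enemy actors, and Heroes when friendly fire is enabled in MainGI.
; Sphere collision switches off briefly at spawn, then its hit event matches the exact class of the struck actor.
; A valid hit fires once, calling GetHit or GetHitServer with a Hero's Damage value, spawning blood at impact and destroying the bullet.
; Other hits print the actor name like all hits, then destroy it after DamageInterval.
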(event OnComponentHit(Sphere1)
  (params (HitComponent :type Primitive%20Component%20Object%20Reference) (OtherActor :type Actor%20Object%20Reference) (OtherComp :type Primitive%20Component%20Object%20Reference) (NormalImpulse :type Vector :default "0, 0, 0") (Hit :type Hit%20Result%20Structure%20%28by%20ref%29))
  (bind _returnvalue (Utilities|GetClass OtherActor))
  (Development|PrintString (Utilities|GetDisplayName OtherActor))
  (bind _asmain_gi (Utilities|Casting|CastToMainGI (Game|GetGameInstance)))
  (if (== _returnvalue "/Game/Gameplay/Blueprints/Enemy.Enemy_C")
    (Utilities|FlowControl|DoOnce false
      (:Completed
        (bind _asenemy (Utilities|Casting|CastToEnemy OtherActor))
        (bind _output_get (Variables|/Game/Gameplay/Blueprints/Enemy.Enemy_C|SetGotHit _asenemy true))
        (Default|GetHit _asenemy _output_get (Variables|/Game/Gameplay/Blueprints/Hero.Hero_C|GetDamage (stale _ashero)))
        (Effects|SpawnEmitteratLocation "/Game/Packages/CartoonMeshParticles/Particles/Bloods/P_BloodExplosion_Short.P_BloodExplosion_Short" (.ImpactPoint (Collision|BreakHitResult Hit)) "0, 0, 0" "1.000000,1.000000,1.000000" true "AutoRelease" :!label _label)))
    (elif (and (Variables|/Game/Gameplay/Online/MainGI.MainGI_C|GetFriendlyFire _asmain_gi) (== _returnvalue "/Game/Gameplay/Blueprints/Hero.Hero_C"))
      (Utilities|FlowControl|DoOnce false
        (:Completed
          (bind _ashero (Utilities|Casting|CastToHero OtherActor))
          (bind _output_get_2 (Variables|/Game/Gameplay/Blueprints/Hero.Hero_C|SetGotHit _ashero true))
          (Default|GetHitServer _ashero (Variables|/Game/Gameplay/Blueprints/Hero.Hero_C|GetDamage _ashero) _output_get_2)
          (goto _label)))
      (else
        (Utilities|FlowControl|Delay (Variables|Default|GetDamageInterval)))))
  (Actor|DestroyActor))

(event EventBeginPlay
  (bind _sphere1 (Variables|Default|GetSphere1))
  (Collision|SetCollisionEnabled _sphere1 "NoCollision")
  (Utilities|FlowControl|Delay 0.01)
  (Collision|SetCollisionEnabled _sphere1 "QueryAndPhysics"))

(fn ConstructionScript)