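; Skeleton enemy that roams the navmesh, chases and attacks the hero, and drops loot on death.
; Far and near overlap volumes switch it between AI MoveTo roaming, chasing and attacking, recoloring a dynamic-material range indicator.
; A weapon-socket collider damages the hero; GetHit lowers health with a brief invulnerability and updates the HUD widget.
; At zero health, it spawns coins or rare health pickups, decrements the spawn manager's count and destroys itself.
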(event OnComponentBeginOverlap(SwordCollision)
  (params (OverlappedComponent :type Primitive%20Component%20Object%20Reference) (OtherActor :type Actor%20Object%20Reference) (OtherComp :type Primitive%20Component%20Object%20Reference) (OtherBodyIndex :type Integer) (bFromSweep :type Boolean) (SweepResult :type Hit%20Result%20Structure%20%28by%20ref%29))
  ;[1 1 1] Hit hero detection
  (if (Utilities|ClassIsChildOf (Utilities|GetClass OtherActor) "/Game/Gameplay/Blueprints/Hero/0_Hero.0_Hero_C")
    (bind _as0_hero (Utilities|Casting|CastTo0_Hero OtherActor))
    (bind _output_get (Variables|/Game/Gameplay/Blueprints/Hero/0_Hero.0_Hero_C|SetGotHit _as0_hero true))
    (Default|GetHit _as0_hero (Variables|Default|GetEnemyDefaultDamage) _output_get)))

(event OnComponentBeginOverlap(nearbyCol)
  (params (OverlappedComponent :type Primitive%20Component%20Object%20Reference) (OtherActor :type Actor%20Object%20Reference) (OtherComp :type Primitive%20Component%20Object%20Reference) (OtherBodyIndex :type Integer) (bFromSweep :type Boolean) (SweepResult :type Hit%20Result%20Structure%20%28by%20ref%29))
  ;[1 1 1] If close hero detection
  (if (Utilities|ClassIsChildOf (Utilities|GetClass OtherActor) "/Game/Gameplay/Blueprints/Hero/0_Hero.0_Hero_C")
    (Variables|Default|SetAttacking true)
    (Rendering|Material|SetVectorParameterValue (Variables|Default|GetDMI_Range) "Color" "(R=1.000000,G=0.000000,B=0.000000,A=1.000000)" :!class /Script/Engine.MaterialInstanceDynamic)))

(event OnComponentEndOverlap(nearbyCol)
  (params (OverlappedComponent :type Primitive%20Component%20Object%20Reference) (OtherActor :type Actor%20Object%20Reference) (OtherComp :type Primitive%20Component%20Object%20Reference) (OtherBodyIndex :type Integer))
  ;[1 1 1] If close hero detection
  (if (Utilities|ClassIsChildOf (Utilities|GetClass OtherActor) "/Game/Gameplay/Blueprints/Hero/0_Hero.0_Hero_C")
    (Utilities|FlowControl|Delay 2.6)
    (Variables|Default|SetAttacking false)
    (CallFunction|ChasePlayer OtherActor)))

(event OnComponentBeginOverlap(FarCol)
  (params (OverlappedComponent :type Primitive%20Component%20Object%20Reference) (OtherActor :type Actor%20Object%20Reference) (OtherComp :type Primitive%20Component%20Object%20Reference) (OtherBodyIndex :type Integer) (bFromSweep :type Boolean) (SweepResult :type Hit%20Result%20Structure%20%28by%20ref%29))
  ;[1 1 1] Far away hero detection
  (if (Utilities|ClassIsChildOf (Utilities|GetClass OtherActor) "/Game/Gameplay/Blueprints/Hero/0_Hero.0_Hero_C")
    (CallFunction|ChasePlayer OtherActor)))

(event OnComponentEndOverlap(FarCol)
  (params (OverlappedComponent :type Primitive%20Component%20Object%20Reference) (OtherActor :type Actor%20Object%20Reference) (OtherComp :type Primitive%20Component%20Object%20Reference) (OtherBodyIndex :type Integer))
  ;[1 1 1] Far away hero detection
  (if (Utilities|ClassIsChildOf (Utilities|GetClass OtherActor) "/Game/Gameplay/Blueprints/Hero/0_Hero.0_Hero_C")
    (CallFunction|Roam)))

(event Custom|Roam
  ;[1 1 1] Roaming event
  (Rendering|Material|SetVectorParameterValue (Variables|Default|GetDMI_Range) "Color" "(R=0.000000,G=0.897796,B=1.000000,A=1.000000)" :!class /Script/Engine.MaterialInstanceDynamic)
  (AI|AIMoveTo self (.RandomLocation (Class|NavigationSystemV1|GetRandomPointinNavigableRadius (Transformation|GetActorLocation) (Variables|Default|Getradius) 0 0)) 0 5.0 false
    (:OnSuccess
      (Utilities|FlowControl|Delay 1.0)
      (CallFunction|Roam))))

(event Custom|LootSprayMulti
  ;[1 1 1] Decides which loot and where to spawn
  (bind _randomlocation (Class|NavigationSystemV1|GetRandomLocationinNavigableRadius (Transformation|GetWorldLocation (Variables|Default|GetStaticMesh1)) (Variables|Default|GetLootSpawnRadius) 0 0))
  (Development|PrintString (Utilities|String|ToString(Vector) _randomlocation))
  (bind _output_get (Variables|Default|SetLootLocation _randomlocation))
  (bind _output_get_2 (Variables|Default|SetGetHealthPickup (> (Math|Random|RandomIntegerinRange 0 10) 9)))
  (if _output_get_2
    (Game|SpawnActorfromClass "/Game/Gameplay/Blueprints/Gameplay/Health.Health_C" (Math|Transform|MakeTransform _output_get "0, 0, 0" "1,1,1") "AlwaysSpawn" 0 0)
    (else
      (Game|SpawnActorfromClass "/Game/Gameplay/Blueprints/Gameplay/Coin.Coin_C" (Math|Transform|MakeTransform _output_get "0, 0, 0" "1,1,1") "AlwaysSpawn" 0 0))))

(event Custom|LootDecider
  ;[1 1 1] Decides which loot and where to spawn
  (for _index (range 0 (- (Variables|Default|GetAmountOfLoot) 1))
    (Networking|SwitchHasAuthority
      (:Authority
        (CallFunction|LootSprayMulti))
      (:Remote
        (CallFunction|LootSprayServer)))))

(event Custom|LootSprayServer
  (CallFunction|LootSprayMulti))

(event Custom|ChasePlayer
  (params (Player :type Actor%20Object%20Reference))
  ;[1 1 1] Chasing player event
  (Rendering|Material|SetVectorParameterValue (Variables|Default|GetDMI_Range) "Color" "(R=1.000000,G=0.341622,B=0.000000,A=1.000000)" :!class /Script/Engine.MaterialInstanceDynamic)
  (AI|AIMoveTo self "0, 0, 0" Player 1.5e+02 false
    (:OnSuccess
      (Utilities|FlowControl|Delay 1.0)
      (CallFunction|ChasePlayer))))

(event Custom|GetHit
  (params (Condition :type Boolean) (B :type Float%20%28single-precision%29))
  ;[1 1 1] GetHit
  (if (and Condition (Variables|Default|GetHittable))
    (Variables|Default|SetHittable false)
    (Variables|Default|SetCurrentHealth (- (Variables|Default|GetCurrentHealth) B))
    (Utilities|FlowControl|Delay 0.7)
    (bind _asenemy_hud (Utilities|Casting|CastToEnemy_HUD (UserInterface|GetUserWidgetObject (Variables|Default|GetEnemyHealthUI))))
    (Variables|/Game/Gameplay/UI/Enemy_HUD.Enemy_HUD_C|SetCurrentHealth_UI _asenemy_hud (Variables|Default|GetCurrentHealth))
    (Variables|Default|SetHittable true)
    (Variables|Default|SetGotHit false)))

(event EventBeginPlay
  ;[1 1 1] Set max hp and start roaming
  (Utilities|FlowControl|Sequence
    (:then_0
      (CallFunction|Roam))
    (:then_1
      (Variables|Default|SetCurrentHealth (Variables|Default|GetMaxHealth))
      (Variables|/Game/Gameplay/UI/Enemy_HUD.Enemy_HUD_C|SetMaxHealth_UI (.AsEnemy%20HUD (Utilities|Casting|CastToEnemy_HUD (UserInterface|GetUserWidgetObject (Variables|Default|GetEnemyHealthUI)))) (Variables|Default|GetMaxHealth)))))

(event EventTick
  (params (DeltaSeconds :type Float%20%28single-precision%29))
  (bind _currenthealth (Variables|Default|GetCurrentHealth))
  (bind _returnvalue (<= _currenthealth 0.0))
  (Utilities|FlowControl|Sequence
    (:then_0
      ;[1 1 1] Dying
      (if _returnvalue
        (Utilities|FlowControl|DoOnce false
          (:Completed
            (Components|Activation|Activate (Variables|Default|GetPS_CoinSpray) false)
            (Utilities|FlowControl|Delay 0.3)
            (CallFunction|LootDecider)
            (Effects|SpawnEmitteratLocation "/Game/Gameplay/Effects/PS_Smoke.PS_Smoke" (- (Transformation|GetWorldLocation (Variables|Default|GetStaticMesh1)) "0, 0,-6.500000"))
            (Utilities|FlowControl|Delay 0.7)
            (Networking|SwitchHasAuthority
              (:Authority
                (bind _returnvalue_2 (Actor|GetActorOfClass "/Game/Gameplay/Blueprints/Enemies/EnemySpawnManager.EnemySpawnManager_C"))
                (Variables|/Game/Gameplay/Blueprints/Enemies/EnemySpawnManager.EnemySpawnManager_C|SetTotalEnemies _returnvalue_2 (- (Variables|/Game/Gameplay/Blueprints/Enemies/EnemySpawnManager.EnemySpawnManager_C|GetTotalEnemies _returnvalue_2) 1))
                (Actor|DestroyActor))
              (:Remote
                (Actor|DestroyActor)))))))
    (:then_1
      ;[1 1 1] if attacking stop moving
      (if (or _returnvalue (Variables|Default|GetAttacking))
        (Components|Movement|StopMovementImmediately (Variables|Character|GetCharacterMovement))))))

(fn ConstructionScript
  (Transformation|AttachComponentToComponent (Variables|Default|GetSwordCollision) (Variables|Character|GetMesh) "Weapon" "KeepRelative" "SnapToTarget" "KeepRelative" true)
  (bind _returnvalue (Rendering|Material|CreateDynamicMaterialInstance "/Game/Gameplay/Materials/M_Range.M_Range" "None" :!class /Script/Engine.KismetMaterialLibrary))
  (bind _output_get (Variables|Default|SetDMI_Range _returnvalue))
  (Rendering|Material|SetMaterial (Variables|Default|GetStaticMesh) 0 _output_get))